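; Player ship for a one-button flying game that moves at constant speed along the world Y axis and tilts with its vertical speed.
; Holding Fly switches Tick gates between climbing and falling, toggling the NSShip effect, with speed and height clamped.
; A timeline animates an idle bob until the first press, which hides the UI tap hint.
; Death forces the release state, notifies the UI and shakes the camera once.
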(event `self.ReceiveBeginPlay`
  (set `self.FirstActorLocation` (`self.K2_GetActorLocation`)))

(event `self.ReceiveTick`
  (params (DeltaSeconds :type "Float (single-precision)"))
  (bind (_returnvalue_x _returnvalue_y _returnvalue_z) (`KismetMathLibrary.BreakVector` (`self.K2_GetActorLocation`)))
  (bind (_returnvalue_x_2 _returnvalue_y_2) (`KismetMathLibrary.BreakVector` (`self.K2_GetActorLocation`)))
  (bind _maxzspeed (`self.MaxZSpeed`))
  (bind _maxzspeed_2 (`self.MaxZSpeed`))
  (bind _startheight (`self.StartHeight`))
  (bind _maxheight (`self.MaxHeight`))
  (bind _maxheight_2 (`self.MaxHeight`))
  (bind _sprite (`self.Sprite`))
  (bind (_returnvalue_x_3 _returnvalue_y_3 _returnvalue_z_2) (`KismetMathLibrary.BreakVector` (+ (`self.K2_GetActorLocation`) (`KismetMathLibrary.MakeVector` 0.0 0.0 (`self.ZSpeed`)))))
  ;[0.5686 1 0.03922] Fly motion
  (`|ExecutionSequence`
    (:`then_0`
      ;[0.5686 1 0.03922] Moves the character to the right
      (if (`self.CanMove?`)
        (`self.K2_AddActorWorldOffset` (0.0 -15.0 0.0))
        ;[0.5884 0.3438 1] Rotates the actor based on the ship's speed
        (if (not (`self.FirstTap?`))
          (`SceneComponent.K2_SetRelativeRotation` _sprite (`KismetMathLibrary.RInterpTo` (`SceneComponent.RelativeRotation` _sprite) (`KismetMathLibrary.MakeRotator` 0.0 (* (`self.ZSpeed`) 4.0)) (`GameplayStatics.GetWorldDeltaSeconds`) 5.4) false false))))
    (:`then_1`
      (`/Engine/EditorBlueprintResources/StandardMacros.Gate` true :!label _label
        (:`Exit`
          (set `self.ZSpeed` (`KismetMathLibrary.FClamp` (+ (`self.ZSpeed`) 0.7) (* _maxzspeed_2 -1.0) _maxzspeed_2))
          (`|ExecutionSequence`
            (:`then_0`
              (`/Engine/EditorBlueprintResources/StandardMacros.DoOnce` false :!label _label_2
                (:`Completed`
                  (`ActorComponent.Activate` (`self.NS_Ship`) false))))
            (:`then_1`
              (`self.K2_SetActorLocation` (`KismetMathLibrary.MakeVector` _returnvalue_x_3 _returnvalue_y_3 (`KismetMathLibrary.FClamp` _returnvalue_z_2 (* _maxheight -1.0) _maxheight)) true :!label _label_3)
              (if (or (<= _returnvalue_z (* _maxheight_2 -1.0)) (>= _returnvalue_z _maxheight_2))
                (set `self.ZSpeed` 0.0)))))))
    (:`then_2`
      (`/Engine/EditorBlueprintResources/StandardMacros.Gate` true :!label _label_4
        (:`Exit`
          (set `self.ZSpeed` (`KismetMathLibrary.FClamp` (+ (`self.ZSpeed`) -0.7) (* _maxzspeed -1.0) _maxzspeed))
          (`|ExecutionSequence`
            (:`then_0`
              (goto _label_3))
            (:`then_1`
              (`/Engine/EditorBlueprintResources/StandardMacros.DoOnce` false :!label _label_5
                (:`Completed`
                  (`ActorComponent.Deactivate` (`self.NS_Ship`)))))))))
    (:`then_3`
      (if (`self.FirstTap?`)
        (`/Engine/EditorBlueprintResources/StandardMacros.DoOnce` false
          (:`Completed`
            (bind (_direction _alpha) (`Timeline|StartPlayerAnim` :!via `PlayFromStart` :!label _label_6)
              (:`Update`
                (bind (_returnvalue_x_4 _returnvalue_y_4 _returnvalue_z_3) (`KismetMathLibrary.BreakVector` (+ (`self.FirstActorLocation`) (`KismetMathLibrary.MakeVector` 0.0 0.0 (`KismetMathLibrary.Lerp` (* _startheight -1.0) _startheight _alpha)))))
                (`self.K2_SetActorLocation` (`KismetMathLibrary.MakeVector` _returnvalue_x_2 _returnvalue_y_2 _returnvalue_z_3))
                (`self.K2_SetActorRotation` (`KismetMathLibrary.RLerp` (`self.StartDownRotation`) (`self.StartUpRotation`) _alpha))))))))))

(event `InputAction|Fly`
  (params (Key :type "Key Structure"))
  ;[0.5686 1 0.03922] Fly motion
  (:`Pressed`
    (if (`self.CanMove?`)
      (`|ExecutionSequence`
        (:`then_0`
          (goto _label :!via `Open`))
        (:`then_1`
          (goto _label_4 :!via `Close`))
        (:`then_2`
          (goto _label_5 :!via `Reset`))
        (:`then_3`
          (`/Engine/EditorBlueprintResources/StandardMacros.DoOnce` false
            (:`Completed`
              (set `self.FirstTap?` false)
              (bind _foundwidgets (`WidgetBlueprintLibrary.GetAllWidgetsOfClass` "/Game/Blueprints/Widgets/UI.UI_C"))
              (`/Game/Blueprints/Widgets/UI.HideTapAdvice` (`|GetArrayItem` _foundwidgets))
              (goto _label_6 :!via `Stop`)))))))
  (:`Released`
    (`|ExecutionSequence` :!label _label_7
      (:`then_0`
        (goto _label :!via `Close`))
      (:`then_1`
        (goto _label_2 :!via `Reset`))
      (:`then_2`
        (goto _label_4 :!via `Open`)))))

(event `Death`
  (`/Engine/EditorBlueprintResources/StandardMacros.DoOnce` false
    (:`Completed`
      (`|ExecutionSequence`
        (:`then_0`
          (goto _label_7))
        (:`then_1`
          (bind _foundwidgets (`WidgetBlueprintLibrary.GetAllWidgetsOfClass` "/Game/Blueprints/Widgets/UI.UI_C"))
          (`/Game/Blueprints/Widgets/UI.Death` (`|GetArrayItem` _foundwidgets))
          (`GameplayStatics.PlayWorldCameraShake` "/Game/Blueprints/DeathCameraShake.DeathCameraShake_C" (`self.K2_GetActorLocation`) 0.0 1000.0 0.0))))))

(fn `UserConstructionScript`)
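; Scrolling background section that chains copies of itself to form an endless level for the player and the menu camera.
; A one-shot overlap on Col spawns the next section at Arrow, for either Player or MenuCamera.
; Player overlaps also spawn Obstacles at both arrows when FirstTap is false.
; After a fixed delay from BeginPlay, the section destroys itself if the player can move or no player exists.
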(event `self.ReceiveBeginPlay`
  ;[0.2708 0.2708 0.2708] Destroys the actor after X time if the player is still playing
  (`KismetSystemLibrary.Delay` 8.0)
  (bind _returnvalue (`GameplayStatics.GetActorOfClass` "/Game/Blueprints/Player.Player_C"))
  (`/Engine/EditorBlueprintResources/StandardMacros.IsValid` _returnvalue
    (:`Is Valid`
      (if (`/Game/Blueprints/Player.CanMove?` _returnvalue)
        (`self.K2_DestroyActor` :!label _label)))
    (:`Is Not Valid`
      (goto _label))))

(event `self.Col.OnComponentBeginOverlap`
  (params (OverlappedComponent :type "PrimitiveComponent Object Reference") (OtherActor :type "Actor Object Reference") (OtherComp :type "PrimitiveComponent Object Reference") (OtherBodyIndex :type Integer) (bFromSweep :type Boolean) (SweepResult :type "HitResult Structure (by ref)"))
  (bind _returnvalue (`SceneComponent.K2_GetComponentToWorld` (`self.Arrow`)))
  ;[0.7373 0.298 0.3373] Spawns another background section when collide
  (bind _asplayer (cast `/Game/Blueprints/Player` OtherActor)
    (:`then`
      (`/Engine/EditorBlueprintResources/StandardMacros.DoOnce` false
        (:`Completed`
          (`|ExecutionSequence`
            (:`then_0`
              (`|SpawnActorFromClass` "Background_C" _returnvalue "Undefined" "OverrideRootScale" null null :!label _label_2))
            (:`then_1`
              (if (not (`/Game/Blueprints/Player.FirstTap?` _asplayer))
                (`|SpawnActorFromClass` "/Game/Blueprints/Obstacles.Obstacles_C" (`KismetMathLibrary.MakeTransform` (.location _returnvalue) (.rotation _returnvalue) (27.5 27.5 27.5)) "Undefined" "OverrideRootScale" null null)
                (`|SpawnActorFromClass` "/Game/Blueprints/Obstacles.Obstacles_C" (`KismetMathLibrary.MakeTransform` (.location (`SceneComponent.K2_GetComponentToWorld` (`self.Arrow1`))) (.rotation (`SceneComponent.K2_GetComponentToWorld` (`self.Arrow1`))) (27.5 27.5 27.5)) "Undefined" "OverrideRootScale" null null)))))))
    (:`CastFailed`
      (cast `/Game/Blueprints/MenuCamera` OtherActor)
      (`/Engine/EditorBlueprintResources/StandardMacros.DoOnce` false
        (:`Completed`
          (goto _label_2))))))

(fn `UserConstructionScript`)
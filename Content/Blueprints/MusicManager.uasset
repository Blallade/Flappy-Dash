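; MusicManager is a Blueprint that controls the game's background music for the menu and gameplay.
; Separate events start or stop the menu and game themes, spawning each as a 2D sound and storing the audio component so it can be stopped later.
; A further event pauses or resumes the game theme through that stored component.
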(event `PlayMenuTheme`
  (params (`Play?` :type Boolean))
  ;[0.5893 0.2185 1] Plays and stop the menu theme
  (if `Play?`
    (bind _returnvalue (`GameplayStatics.SpawnSound2D` "/Game/Audio/The_scrap_boy_fragment.The_scrap_boy_fragment" 1.0 1.0 0.0 null))
    (set `self.MenuTheme` _returnvalue)
    (else
      (`AudioComponent.Stop` (`self.MenuTheme`)))))

(event `PlayGameTheme`
  (params (`Play?` :type Boolean))
  ;[0.5893 0.2185 1] Plays and stop the game theme
  (if `Play?`
    (bind _returnvalue (`GameplayStatics.SpawnSound2D` "/Game/Audio/The_undertaker_s_daughter_fragment.The_undertaker_s_daughter_fragment" 1.0 1.0 0.0 null))
    (set `self.GameTheme` _returnvalue)
    (else
      (`AudioComponent.Stop` (`self.GameTheme`)))))

(event `PauseGameTheme`
  (params (`Pause?` :type Boolean))
  ;[0.5893 0.2185 1] Pauses the game theme
  (`AudioComponent.SetPaused` (`self.GameTheme`) `Pause?`))

(fn `UserConstructionScript`)